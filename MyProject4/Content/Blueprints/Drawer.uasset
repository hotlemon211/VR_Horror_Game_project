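; Drawer actor that slides along one axis while grabbed by a motion controller.
; GrabComponent's grab event stores the controller and starts a fast looping timer, and its drop event clears both.
; Each timer tick adds the controller's Y offset relative to the Capsule to the Capsule's relative Y, clamped between the first two spline points' local Y values.
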(event OnGrabbed(GrabComponent)
  (params (Motion%20Controller :type Motion%20Controller%20Component%20Object%20Reference))
  (Variables|Default|SetMotion%20Controller Motion%20Controller)
  (bind _returnvalue (Utilities|Time|SetTimerbyFunctionName 0 "UpdateLocation" 0.01 true))
  (Variables|Default|SetTimer _returnvalue))

(event OnDropped(GrabComponent)
  (Utilities|Time|ClearandInvalidateTimerbyHandle (Variables|Default|GetTimer))
  (Variables|Default|SetMotion%20Controller 0))

(event EventBeginPlay)

(event Collision|EventActorBeginOverlap
  (params (OtherActor :type Actor%20Object%20Reference)))

(event EventTick
  (params (DeltaSeconds :type Float%20%28single-precision%29)))

(fn ConstructionScript)

(fn UpdateLocation
  (bind _capsule (Variables|Default|GetCapsule))
  (bind _spline (Variables|Default|GetSpline))
  (bind _relativelocation (Variables|/Script/Engine.SceneComponent|GetRelativeLocation _capsule))
  (Transformation|SetRelativeLocation _capsule (Math|Vector|MakeVector (.x _relativelocation) (Math|Float|Clamp(Float) (+ (.y _relativelocation) (.y (.location (Math|Transform|MakeRelativeTransform (Transformation|GetWorldTransform (Variables|Default|GetMotion%20Controller)) (Transformation|GetWorldTransform (Variables|Default|GetCapsule)))))) (.y (Spline|GetLocationatSplinePoint _spline 0 "Local")) (.y (Spline|GetLocationatSplinePoint _spline 1 "Local"))) (.z _relativelocation)) false false))