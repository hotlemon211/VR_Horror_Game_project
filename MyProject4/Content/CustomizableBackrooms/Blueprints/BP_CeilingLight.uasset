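; BP_CeilingLight is a Backrooms ceiling light fixture that flickers continuously during play.
; After a short random delay on BeginPlay, the Flicker event runs a chain of randomly timed off/on toggles, then calls itself to repeat indefinitely.
; TurnOff and TurnOn switch the mesh's Emissive Intensity material parameter and the SpotLight's visibility together, so the panel glow matches the cast light.
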(event Custom|Turn%20Off
  (Rendering|Material|SetScalarParameterValueonMaterials (Variables|Default|GetSM_BigCeilingLights) "Emissive Intensity" 0.0)
  (Rendering|SetVisibility (Variables|Default|GetSpotLight) false false))

(event Custom|Turn%20On
  (Rendering|Material|SetScalarParameterValueonMaterials (Variables|Default|GetSM_BigCeilingLights) "Emissive Intensity" 1.0)
  (Rendering|SetVisibility (Variables|Default|GetSpotLight) true false))

(event Custom|Flicker
  (bind _returnvalue (Math|Random|RandomFloatinRange 0.5 2.0))
  (Utilities|FlowControl|Delay (Math|Random|RandomFloatinRange 0.1 5.0))
  (CallFunction|TurnOff)
  (Utilities|FlowControl|Delay (Math|Random|RandomFloatinRange 0.1 0.25))
  (CallFunction|Turnon)
  (Utilities|FlowControl|Delay (Math|Random|RandomFloatinRange 0.1 0.25))
  (CallFunction|TurnOff)
  (Utilities|FlowControl|Delay (Math|Random|RandomFloatinRange 0.1 1.0))
  (CallFunction|Turnon)
  (Utilities|FlowControl|Delay (Math|Random|RandomFloatinRange 0.1 0.2))
  (CallFunction|TurnOff)
  (Utilities|FlowControl|Delay (Math|Random|RandomFloatinRange 0.1 0.25))
  (CallFunction|Turnon)
  (Utilities|FlowControl|Delay _returnvalue)
  (CallFunction|TurnOff)
  (Utilities|FlowControl|Delay _returnvalue)
  (CallFunction|Turnon)
  (CallFunction|Flicker))

(event EventBeginPlay
  (bind _returnvalue (Math|Random|RandomFloatinRange 0.5 2.0))
  (Utilities|FlowControl|Delay (Math|Random|RandomFloatinRange 0.1 0.5))
  (Utilities|FlowControl|Delay (Math|Random|RandomFloatinRange 0.1 5.0))
  (CallFunction|TurnOff)
  (Utilities|FlowControl|Delay (Math|Random|RandomFloatinRange 0.1 0.25))
  (CallFunction|Turnon)
  (Utilities|FlowControl|Delay (Math|Random|RandomFloatinRange 0.1 0.25))
  (CallFunction|TurnOff)
  (Utilities|FlowControl|Delay (Math|Random|RandomFloatinRange 0.1 1.0))
  (CallFunction|Turnon)
  (Utilities|FlowControl|Delay (Math|Random|RandomFloatinRange 0.1 0.2))
  (CallFunction|TurnOff)
  (Utilities|FlowControl|Delay (Math|Random|RandomFloatinRange 0.1 0.25))
  (CallFunction|Turnon)
  (Utilities|FlowControl|Delay _returnvalue)
  (CallFunction|TurnOff)
  (Utilities|FlowControl|Delay _returnvalue)
  (CallFunction|Turnon)
  (CallFunction|Flicker))

(fn ConstructionScript)